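; BP_EnergySphere is a short-lived wandering sphere actor that scales in on spawn and scales out before destroying itself.
; Tick moves it forward while spinning it by a scaled random rotator, re-rolled at random intervals to vary its path.
; Timelines drive both scale animations, with wink-out triggered by a lifespan timer or a SphereVolume overlap.
; The overlap check skips wink-out only when already winking out and touching the DefaultPawn.
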(event `WinkIn`
  (bind (_direction _scale) (`Timeline|WinkInTimeline`)
    (:`Update`
      (`SceneComponent.SetWorldScale3D` (`self.EnergySphere`) _scale))))

(event `WinkOut`
  (set `self.isWinkingOut` true)
  (bind (_direction _scale) (`Timeline|WinkOutTimeline`)
    (:`Update`
      (`SceneComponent.SetWorldScale3D` (`self.EnergySphere`) (`KismetMathLibrary.Conv_DoubleToVector` _scale)))
    (:`Finished`
      (`self.K2_DestroyActor`))))

(event `OnComponentBeginOverlap_Event`
  (params (OverlappedComponent :type "PrimitiveComponent Object Reference") (OtherActor :type "Actor Object Reference") (OtherComp :type "PrimitiveComponent Object Reference") (OtherBodyIndex :type Integer) (bFromSweep :type Boolean) (SweepResult :type "HitResult Structure (by ref)"))
  (bind _returnvalue (`GameplayStatics.GetActorOfClass` "/Script/Engine.DefaultPawn"))
  (`|ExecutionSequence`
    (:`then_0`
      (bind _returnvalue_2 (== _returnvalue OtherActor))
      (if (not (and (`self.isWinkingOut`) _returnvalue_2))
        (`self.WinkOut`)
        (`KismetSystemLibrary.PrintString` (`KismetStringLibrary.Concat_StrStr` "Wink out triggered for: " (`KismetSystemLibrary.GetDisplayName` self)))))
    (:`then_1`
      (`KismetSystemLibrary.PrintString` (`KismetStringLibrary.Concat_StrStr` "Default pawn overlapped: " (`KismetStringLibrary.Conv_BoolToString` _returnvalue_2) ", with: " (`KismetSystemLibrary.GetDisplayName` self))))))

(event `self.ReceiveBeginPlay`
  (`self.InitVariables`)
  (`self.WinkIn`)
  (`KismetSystemLibrary.K2_SetTimerDelegate` (delegate `WinkOut`) (`self.LifeSpan`))
  (add `PrimitiveComponent.OnComponentBeginOverlap` (`self.SphereVolume`) (delegate `OnComponentBeginOverlap_Event`)))

(event `self.ReceiveTick`
  (params (DeltaSeconds :type "Float (single-precision)"))
  (set `self.CurrentDeltaSeconds` DeltaSeconds)
  (`|ExecutionSequence`
    (:`then_1`
      (`self.MoveEnergySphere`))
    (:`then_2`
      (if (< (`self.TimeSinceLastChange`) (`self.ChangeInterval`))
        (`self.UpdateTimeSinceLastChange`)
        (else
          (`self.InitVariables`)))
      (`self.RotateEnergySphere`))))

(fn `InitVariables`
  (set `self.TimeSinceLastChange` 0.0)
  (set `self.ChangeInterval` (`KismetMathLibrary.RandomFloatInRange` (`self.ChangeIntervalMin`) (`self.ChangeIntervalMax`)))
  (set `self.TargetRotation` (`KismetMathLibrary.RandomRotator` false)))

(fn `MoveEnergySphere`
  (`self.K2_AddActorWorldOffset` (* (`self.GetActorForwardVector`) (* (`self.CurrentDeltaSeconds`) (`self.MovementSpeed`)))))

(fn `PrintDebugInfo`
  (`KismetSystemLibrary.PrintString` (`KismetStringLibrary.Concat_StrStr` "Time since last change: " (`KismetStringLibrary.Conv_DoubleToString` (`self.TimeSinceLastChange`))) true true (struct :`G` 0.66 :`B` 1.0 :`A` 1.0) 0.0)
  (`KismetSystemLibrary.PrintString` (`KismetStringLibrary.Concat_StrStr` "Change interval: " (`KismetStringLibrary.Conv_DoubleToString` (`self.ChangeInterval`))) true true (struct :`G` 0.66 :`B` 1.0 :`A` 1.0) 0.0)
  (`KismetSystemLibrary.PrintString` (`KismetStringLibrary.Concat_StrStr` "Actor rotation: " (`KismetStringLibrary.Conv_RotatorToString` (`self.K2_GetActorRotation`))) true true (struct :`G` 0.66 :`B` 1.0 :`A` 1.0) 0.0)
  (`KismetSystemLibrary.PrintString` (`KismetStringLibrary.Concat_StrStr` "Target rotation: " (`KismetStringLibrary.Conv_RotatorToString` (`self.TargetRotation`))) true true (struct :`G` 0.66 :`B` 1.0 :`A` 1.0) 0.0)
  (`KismetSystemLibrary.PrintString` (`KismetStringLibrary.Concat_StrStr` "Rotation speed: " (`KismetStringLibrary.Conv_DoubleToString` (`self.RotationSpeed`))) true true (struct :`G` 0.66 :`B` 1.0 :`A` 1.0) 0.0))

(fn `RotateEnergySphere`
  (`self.K2_AddActorWorldRotation` (* (* (`self.TargetRotation`) (`self.CurrentDeltaSeconds`)) (`self.RotationScaleFactor`))))

(fn `UpdateTimeSinceLastChange`
  (set `self.TimeSinceLastChange` (+ (`self.TimeSinceLastChange`) (`self.CurrentDeltaSeconds`))))

(fn `UserConstructionScript`)