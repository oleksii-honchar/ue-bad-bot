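; BP_Utilities holds debug helper functions for printing an actor's location on screen.
; PrintActorLocation shows the display name and location for a long duration, using a key built from the name and its hash so repeat calls replace that actor's previous message.
; HashString computes that hash with a djb2-style multiply-by-33 accumulation over the string's characters.
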(fn `HashString`
  (params (InputString :type String))
  (returns (Hash :type Integer))
  (locals (Accumulator :type Integer :default 5381))
  (for _array_element (`KismetStringLibrary.GetCharacterArrayFromString` InputString)
    (bind _output_get (set `local.Accumulator` (+ (* (`local.Accumulator`) 33) (`KismetStringLibrary.GetCharacterAsNumber` _array_element)))))
  (return _output_get))

(fn `PrintActorLocation`
  (params (TargetActor :type "Actor Object Reference"))
  (bind _returnvalue (`KismetSystemLibrary.GetDisplayName` TargetActor))
  (bind _hash (`self.HashString` _returnvalue))
  (`KismetSystemLibrary.PrintString` null (`KismetStringLibrary.Concat_StrStr` _returnvalue ":" (`KismetStringLibrary.Conv_VectorToString` (`Actor.K2_GetActorLocation` TargetActor))) true true (struct :`G` 0.66 :`B` 1.0 :`A` 1.0) 900.0 (`KismetStringLibrary.Conv_StringToName` (`KismetStringLibrary.Concat_StrStr` _returnvalue "-" (`KismetStringLibrary.Conv_IntToString` _hash)))))